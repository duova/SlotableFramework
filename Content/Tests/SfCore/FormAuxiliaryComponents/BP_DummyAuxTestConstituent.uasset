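; Test dummy constituent for SfCore form auxiliary components, exercising stats, resources, queries and input-driven actions.
; On server initialization it binds a test query that sets a called flag, and adds additive modifiers to the test resource increase and decrease stats, removing them on deinitialization.
; Input down executes an action, forwarding the predictable-context flag, and the constituent action predictively sets the test resource to a fixed value.
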(event Custom|OnTestQuery
  (Variables|Default|SetTestQueryCalled true))

(event EventServerInitialize
  (params (bInIsPredictableContext :type Boolean))
  (Class|TestQuery|BindTestQuery 0 (delegate Custom|OnTestQuery))
  (bind _output_get (Variables|Default|SetForm%20Stat (Variables|/Script/SfCore.FormCoreComponent|GetFormStat (Class|Constituent|GetFormCoreComponent))))
  (bind _returnvalue (Class|FormStatComponent|ServerAddStatModifier _output_get "(TagName=\"Stat.TestResourceIncrease\")" "Additive" 2.0))
  (Variables|Default|SetTestResourceIncreaseModifier _returnvalue)
  (bind _returnvalue_2 (Class|FormStatComponent|ServerAddStatModifier (Variables|Default|GetForm%20Stat) "(TagName=\"Stat.TestResourceDecrease\")" "Additive" 1.0))
  (Variables|Default|SetTestResourceDecreaseModifier _returnvalue_2))

(event EventServerDeinitialize
  (params (bInIsPredictableContext :type Boolean))
  (Class|FormStatComponent|ServerRemoveStatModifier (Variables|Default|GetForm%20Stat) (Variables|Default|GetTestResourceIncreaseModifier) "Additive")
  (Class|FormStatComponent|ServerRemoveStatModifier (Variables|Default|GetForm%20Stat) (Variables|Default|GetTestResourceDecreaseModifier) "Additive"))

(event EventOnInputDown
  (params (bInIsPredictableContext :type Boolean))
  (Class|Constituent|ExecuteAction 1 bInIsPredictableContext))