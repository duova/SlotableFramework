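; Multiplayer test of the SfCore form auxiliary components: stats, resources and health.
; It registers procedures tagged by net role, spawning and possessing a dummy character, then asserting values on server, autonomous and simulated proxies.
; It checks stat modifiers, resource prediction via injected Enhanced Input, and constant resource and health changes after timed waits.
; Lastly, it kills the form to validate the death handler's health-change data.
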(event Custom|Spawn%20form%20character,%20cache%20elements,%20and%20pass%20ownership
  (bind _returnvalue (Class|SfObject|SpawnActorinOwnerWorld (Variables|Default|GetFormCharacterClass) (Variables|Default|GetLocation) (Variables|Default|GetRotation)))
  (bind _asbp_dummy_aux_character (Utilities|Casting|CastToBP_DummyAuxCharacter _returnvalue))
  (bind _output_get (Variables|Default|SetFormCharacter _asbp_dummy_aux_character))
  (Pawn|Possess (Class|SfTest|GetAutonomousPlayerController) _output_get)
  (bind _output_get_2 (Variables|Default|SetForm%20Core (Variables|/Script/SfCore.FormCharacter|GetFormCore (Variables|Default|GetFormCharacter))))
  (bind _output_get_3 (Variables|Default|SetInventory (Utilities|Array|Get(acopy) (Class|FormCoreComponent|GetInventories _output_get_2))))
  (bind _output_get_4 (Variables|Default|SetSlotable (Utilities|Array|Get(acopy) (Class|Inventory|GetSlotables _output_get_3))))
  (bind _asbp_dummy_aux_test_constituent (Utilities|Casting|CastToBP_DummyAuxTestConstituent (Utilities|Array|Get(acopy) (Class|Slotable|GetConstituents _output_get_4))))
  (Variables|Default|SetConstituent _asbp_dummy_aux_test_constituent))

(event Custom|Check%20if%20test%20query%20was%20called
  (Class|SfTest|AssertBool (Variables|/Game/Tests/SfCore/FormAuxiliaryComponents/BP_DummyAuxTestConstituent.BP_DummyAuxTestConstituent_C|GetTestQueryCalled (Variables|Default|GetConstituent)) true "Test query"))

(event Custom|Verify%20constant%20resource%20changes
  (Class|SfTest|AssertFloat (Class|FormResourceComponent|GetResourceValue (Variables|/Script/SfCore.FormCoreComponent|GetFormResource (Variables|Default|GetForm%20Core)) "(TagName=\"Resource.Test\")") 53.0 57.0 "Constant resource changes"))

(event Custom|Verify%20health%20and%20constant%20changes%20synced%20to%20autonomous
  (Class|SfTest|AssertFloat (Class|SfHealthComponent|GetHealth (Variables|/Script/SfCore.FormCoreComponent|GetSfHealth (Variables|Default|GetForm%20Core))) 63.0 67.0 "Verify health and constant changes synced to autonomous"))

(event Custom|Verify%20health%20and%20constant%20changes%20synced%20to%20simulated
  (Class|SfTest|AssertFloat (Class|SfHealthComponent|GetHealth (Variables|/Script/SfCore.FormCoreComponent|GetSfHealth (Variables|Default|GetForm%20Core))) 63.0 67.0 "Verify health and constant changes synced to simulated"))

(event Custom|Kill%20form%20and%20verify%20that%20death%20handler%20is%20called%20with%20the%20correct%20data
  (bind _formcharacter (Variables|Default|GetFormCharacter))
  (bind _deathhealthchangedata (Variables|/Game/Tests/SfCore/FormAuxiliaryComponents/BP_DummyAuxCharacter.BP_DummyAuxCharacter_C|GetDeathHealthChangeData _formcharacter))
  (bind _output (Utilities|Array|Get(acopy) _deathhealthchangedata))
  (bind (_invalue _outvalue _source _processors) (Utilities|Struct|BreakHealthChangeData _output))
  (Class|SfHealthComponent|ApplyHealthChange (Variables|/Script/SfCore.FormCoreComponent|GetSfHealth (Variables|Default|GetForm%20Core)) -1e+02 0 (Variables|Default|GetTrueHealthProcessor))
  (Class|SfTest|AssertBool (Variables|/Game/Tests/SfCore/FormAuxiliaryComponents/BP_DummyAuxCharacter.BP_DummyAuxCharacter_C|GetIsDead (Variables|Default|GetFormCharacter)) true "Form calling death handler")
  (Class|SfTest|AssertInt (Utilities|Array|Length _deathhealthchangedata) 2 2 "HealthChangeData length")
  (Class|SfTest|AssertFloat _outvalue -106.0 -104.0 "HealthChangeData value") ; -105 damage dealt because 100 to 0 health but there was 5 health worth of healing in between
  (Class|SfTest|GenericAssert (== (Utilities|Array|Get(acopy) _processors) "/Game/Tests/SfCore/FormAuxiliaryComponents/BP_TrueHealthProcessor.BP_TrueHealthProcessor_C") "HealthProcessor given on death is correct" "HealthProcessor given on death is incorrect"))

(event Custom|Verify%20on%20autonomous%20after%20waiting%20for%20tick
  (Class|SfTest|AssertFloat (Class|FormResourceComponent|GetResourceValue (Variables|/Script/SfCore.FormCoreComponent|GetFormResource (Class|Constituent|GetFormCoreComponent (Variables|Default|GetConstituent))) "(TagName=\"Resource.Test\")") 48.0 52.0 "Predictive resource set autonomous"))

(event Custom|Verify%20stat%20modifers%20work%20on%20server
  (Class|SfTest|AssertFloat (Class|FormStatComponent|GetStat (Variables|/Game/Tests/SfCore/FormAuxiliaryComponents/BP_DummyAuxCharacter.BP_DummyAuxCharacter_C|GetFormStat (Variables|Default|GetFormCharacter)) "(TagName=\"Stat.TestResourceIncrease\")") 2.0 2.0 "TestResourceIncreaseModifer Server")
  (Class|SfTest|AssertFloat (Class|FormStatComponent|GetStat (Variables|/Game/Tests/SfCore/FormAuxiliaryComponents/BP_DummyAuxCharacter.BP_DummyAuxCharacter_C|GetFormStat (Variables|Default|GetFormCharacter)) "(TagName=\"Stat.TestResourceDecrease\")") 1.0 1.0 "TestResourceDecreaseModifer Server"))

(event Custom|Verify%20starting%20health%20on%20server
  (Class|SfTest|AssertFloat (Class|SfHealthComponent|GetHealth (Variables|/Script/SfCore.FormCoreComponent|GetSfHealth (Variables|Default|GetForm%20Core))) 99.0 101.0 "Verify starting health on server"))

(event Custom|Verify%20stat%20mods%20synced%20to%20autonomous
  (Class|SfTest|AssertFloat (Class|FormStatComponent|GetStat (Variables|/Game/Tests/SfCore/FormAuxiliaryComponents/BP_DummyAuxCharacter.BP_DummyAuxCharacter_C|GetFormStat (Variables|Default|GetFormCharacter)) "(TagName=\"Stat.TestResourceIncrease\")") 2.0 2.0 "TestResourceIncreaseModifer Autonomous")
  (Class|SfTest|AssertFloat (Class|FormStatComponent|GetStat (Variables|/Game/Tests/SfCore/FormAuxiliaryComponents/BP_DummyAuxCharacter.BP_DummyAuxCharacter_C|GetFormStat (Variables|Default|GetFormCharacter)) "(TagName=\"Stat.TestResourceDecrease\")") 1.0 1.0 "TestResourceDecreaseModifer Autonomous"))

(event Custom|Deduct%20health%20on%20server
  (bind _truehealthprocessor (Variables|Default|GetTrueHealthProcessor))
  (bind _form_core (Variables|Default|GetForm%20Core))
  (bind _sfhealth (Variables|/Script/SfCore.FormCoreComponent|GetSfHealth _form_core))
  (Class|SfHealthComponent|ApplyHealthChange _sfhealth -1e+01 0 _truehealthprocessor)
  (Class|SfHealthComponent|ApplyHealthChange _sfhealth -1e+01 0 _truehealthprocessor)
  (Class|SfHealthComponent|ApplyHealthChange _sfhealth -1e+01 0 _truehealthprocessor)
  (Class|SfHealthComponent|ApplyHealthChange _sfhealth -1e+01 0 _truehealthprocessor)
  (Class|SfTest|AssertFloat (Class|SfHealthComponent|GetHealth _sfhealth) 59.0 61.0 "Verify health change on server"))

(event Custom|Verify%20stat%20mods%20synced%20to%20simulated
  (Class|SfTest|AssertFloat (Class|FormStatComponent|GetStat (Variables|/Game/Tests/SfCore/FormAuxiliaryComponents/BP_DummyAuxCharacter.BP_DummyAuxCharacter_C|GetFormStat (Variables|Default|GetFormCharacter)) "(TagName=\"Stat.TestResourceIncrease\")") 2.0 2.0 "TestResourceIncreaseModifer Simulated")
  (Class|SfTest|AssertFloat (Class|FormStatComponent|GetStat (Variables|/Game/Tests/SfCore/FormAuxiliaryComponents/BP_DummyAuxCharacter.BP_DummyAuxCharacter_C|GetFormStat (Variables|Default|GetFormCharacter)) "(TagName=\"Stat.TestResourceDecrease\")") 1.0 1.0 "TestResourceDecreaseModifer Simulated"))

(event Custom|Predictively%20modify%20resource%20value
  (bind _asplayer_controller (Utilities|Casting|CastToPlayerController (Pawn|GetController (Variables|Default|GetFormCharacter))))
  (Class|EnhancedInputSubsystemInterface|InjectInputVectorforAction (PlayerController|LocalPlayerSubsystems|GetEnhancedInputLocalPlayerSubsystem _asplayer_controller) "/Game/Tests/SfCore/FormCharacterComponent/IA_Test1.IA_Test1" "1.000000,0.000000,0.000000"))

(event Custom|Verify%20on%20server
  (Class|SfTest|AssertFloat (Class|FormResourceComponent|GetResourceValue (Variables|/Script/SfCore.FormCoreComponent|GetFormResource (Variables|Default|GetForm%20Core)) "(TagName=\"Resource.Test\")") 48.0 52.0 "Predictive resource set server"))

(event Custom|Verify%20on%20simulated
  (Class|SfTest|AssertFloat (Class|FormResourceComponent|GetResourceValue (Variables|/Script/SfCore.FormCoreComponent|GetFormResource (Variables|Default|GetForm%20Core)) "(TagName=\"Resource.Test\")") 48.0 52.0 "Predictive resource set simulated"))

(event EventBlueprintRegisterProcedures
  (Class|SfTest|AddProcedure (delegate Custom|Spawn%20form%20character,%20cache%20elements,%20and%20pass%20ownership) "ROLE_Authority" 0.2)
  (Class|SfTest|AddProcedure (delegate Custom|Check%20if%20test%20query%20was%20called) "ROLE_Authority" 0.0)
  (Class|SfTest|AddProcedure (delegate Custom|Verify%20stat%20modifers%20work%20on%20server) "ROLE_Authority" 0.0)
  (Class|SfTest|AddProcedure (delegate Custom|Verify%20stat%20mods%20synced%20to%20autonomous) "ROLE_AutonomousProxy" 0.0)
  (Class|SfTest|AddProcedure (delegate Custom|Verify%20stat%20mods%20synced%20to%20simulated) "ROLE_SimulatedProxy" 0.0)
  (Class|SfTest|AddProcedure (delegate Custom|Predictively%20modify%20resource%20value) "ROLE_AutonomousProxy" 0.0)
  (Class|SfTest|AddProcedure (delegate Custom|Verify%20on%20autonomous%20after%20waiting%20for%20tick) "ROLE_AutonomousProxy" 0.0)
  (Class|SfTest|AddProcedure (delegate Custom|Verify%20on%20server) "ROLE_Authority" 0.0)
  (Class|SfTest|AddProcedure (delegate Custom|Verify%20on%20simulated) "ROLE_SimulatedProxy" 5.0)
  (Class|SfTest|AddProcedure (delegate Custom|Verify%20constant%20resource%20changes) "ROLE_Authority" 0.0)
  (Class|SfTest|AddProcedure (delegate Custom|Verify%20starting%20health%20on%20server) "ROLE_Authority" 0.0)
  (Class|SfTest|AddProcedure (delegate Custom|Deduct%20health%20on%20server) "ROLE_Authority" 5.0)
  (Class|SfTest|AddProcedure (delegate Custom|Verify%20health%20and%20constant%20changes%20synced%20to%20autonomous) "ROLE_AutonomousProxy" 0.0)
  (Class|SfTest|AddProcedure (delegate Custom|Verify%20health%20and%20constant%20changes%20synced%20to%20simulated) "ROLE_SimulatedProxy" 0.0)
  (Class|SfTest|AddProcedure (delegate Custom|Kill%20form%20and%20verify%20that%20death%20handler%20is%20called%20with%20the%20correct%20data) "ROLE_Authority" 0.0))