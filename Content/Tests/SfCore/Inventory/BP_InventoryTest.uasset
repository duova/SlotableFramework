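; Multiplayer functional test for SfCore inventories, covering slotable operations and shared cards on a spawned pawn's FormCore.
; Registers ordered procedures by net role: Authority creates inventories and mutates them, while AutonomousProxy asserts the results replicated to the client.
; Slotable tests cover add, remove, set, insert, swap and cross-inventory trade, with some bound callbacks checked through captured variables.
; Card tests cover default, removal and timed addition, using a post-procedure wait to confirm client-side expiry.
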(event Custom|Create%20form%20pawn%20and%20inventory
  (bind _returnvalue (Class|SfObject|SpawnActorinOwnerWorld (Variables|Default|GetPawnClass) (Math|Vector|MakeVector 0.0 0.0 0.0) (Math|Rotator|MakeRotator 0.0 0.0 0.0)))
  (bind _output_get (Variables|Default|SetPawn _returnvalue))
  (bind _output_get_2 (Variables|Default|SetFormCore (Actor|GetComponentbyClass _output_get "/Script/SfCore.FormCoreComponent")))
  (Class|SfTest|GenericAssert (Utilities|IsValid (Utilities|Array|Get(acopy) (Class|FormCoreComponent|GetInventories _output_get_2))) "Default inventory successfully created." "Failed to create default inventory.")
  (bind _returnvalue_2 (Class|FormCoreComponent|ServerAddInventory (Variables|Default|GetFormCore) (Variables|Default|GetIn%20Inventory%20Class)))
  (Variables|Default|SetCreatedInventory _returnvalue_2))

(event Custom|Check%20default%20card%20added
  (Class|SfTest|AssertBool (Class|Inventory|HasSharedCard (Variables|Default|GetCreatedInventory) (Variables|Default|GetIn%20Card%20Class)) true "Check default card"))

(event Custom|Check%20OwningFormCore%20synced%20to%20client
  (Class|SfTest|GenericAssert (== (Variables|/Script/SfCore.Inventory|GetOwningFormCore (Variables|Default|GetCreatedInventory)) (Variables|Default|GetFormCore)) "OwnedFormCore synced to client" "OwnedFormCore failed to sync to client"))

(event Custom|Check%20default%20slotable%20synced%20to%20client
  (Class|SfTest|GenericAssert (Utilities|IsValid (Utilities|Array|Get(acopy) (Class|Inventory|GetSlotables (Variables|Default|GetCreatedInventory)))) "Default slotable synced to client" "Default slotable failed to sync to client"))

(event Custom|Add%20slotable
  (bind _createdinventory (Variables|Default|GetCreatedInventory))
  (bind _in_slotable_class (Variables|Default|GetIn%20Slotable%20Class))
  (Class|Inventory|ServerBindonAddSlotable _createdinventory _in_slotable_class (delegate Custom|OnAddSlotable))
  (bind _returnvalue (Class|Inventory|ServerAddSlotable _createdinventory _in_slotable_class))
  (Class|SfTest|GenericAssert (and (Utilities|IsValid (stale Custom|OnAddSlotable _output_get)) (== _returnvalue (stale Custom|OnAddSlotable _output_get))) "OnAddSlotable called with correct slotable" "OnAddSlotable called with incorrect slotable"))

(event Custom|Try%20GetSlotablesOfClass%20on%20client
  (Class|SfTest|AssertInt (Utilities|Array|Length (Class|Inventory|GetSlotablesOfClass (Variables|Default|GetCreatedInventory) (Variables|Default|GetIn%20Slotable%20Class))) 1 1 "Verify GetSlotablesOfClass"))

(event Custom|RemoveSlotableByIndex
  (bind _createdinventory (Variables|Default|GetCreatedInventory))
  (Class|Inventory|ServerBindonRemoveSlotable (Variables|Default|GetCreatedInventory) (Variables|Default|GetIn%20Slotable%20Class) (delegate Custom|OnRemoveSlotable))
  (Class|Inventory|ServerRemoveSlotablebyIndex _createdinventory 1 true)
  (Class|SfTest|AssertInt (Utilities|Array|Length (Class|Inventory|GetSlotables _createdinventory)) 1 1 "Remove slotable by index")
  (Class|SfTest|GenericAssert (stale Custom|OnRemoveSlotable _output_get) "OnRemoveSlotable called" "OnRemoveSlotable not called"))

(event Custom|Card%20removal
  (Class|Inventory|BindonRemoveSharedCard (Variables|Default|GetCreatedInventory) (Variables|Default|GetIn%20Card%20Class) (delegate Custom|OnRemoveSharedCard))
  (Class|Inventory|ServerRemoveSharedCard (Variables|Default|GetCreatedInventory) (Variables|Default|GetIn%20Card%20Class))
  (Class|SfTest|AssertBool (Class|Inventory|HasSharedCard (Variables|Default|GetCreatedInventory) (Variables|Default|GetIn%20Card%20Class)) false "Remove shared card")
  (Class|SfTest|AssertBool (Variables|Default|GetCard%20removed) true "On card removed"))

(event Custom|Set%20slotable
  (Class|Inventory|ServerSetSlotable (Variables|Default|GetCreatedInventory) (Variables|Default|GetEmptySlotable) 0 false)
  (Class|SfTest|AssertInt (Class|Inventory|SlotableCount (Variables|Default|GetCreatedInventory) (Variables|Default|GetEmptySlotable)) 1 1 "Set slotable"))

(event Custom|Insert%20slotable
  (bind _createdinventory (Variables|Default|GetCreatedInventory))
  (Class|Inventory|ServerInsertSlotable _createdinventory (Variables|Default|GetIn%20Slotable%20Class))
  (Class|SfTest|GenericAssert (== (Utilities|GetClass (Utilities|Array|Get(acopy) (Class|Inventory|GetSlotables _createdinventory) 1)) (Variables|Default|GetEmptySlotable)) "Slotable inserted" "Slotable failed to insert"))

(event Custom|Swap%20slotable
  (bind _createdinventory (Variables|Default|GetCreatedInventory))
  (bind _returnvalue (Class|Inventory|GetSlotables _createdinventory))
  (Class|Inventory|ServerSwapSlotables _createdinventory (Utilities|Array|Get(acopy) _returnvalue) (Utilities|Array|Get(acopy) _returnvalue 1))
  (Class|SfTest|GenericAssert (== (Utilities|GetClass (Utilities|Array|Get(acopy) (Class|Inventory|GetSlotables (Variables|Default|GetCreatedInventory)))) (Variables|Default|GetEmptySlotable)) "Slotables swapped" "Slotables failed to swap"))

(event Custom|Trade%20slotables%20between%20inventories
  (bind _returnvalue (Class|FormCoreComponent|ServerAddInventory (Variables|Default|GetFormCore) (Variables|Default|GetIn%20Inventory%20Class)))
  (Class|Inventory|ServerTradeSlotablesBetweenInventories _returnvalue (Utilities|Array|Get(acopy) (Class|Inventory|GetSlotables (Variables|Default|GetCreatedInventory))) (Utilities|Array|Get(acopy) (Class|Inventory|GetSlotables _returnvalue))))

(event Custom|Verify%20changes%20on%20client
  (bind _createdinventory (Variables|Default|GetCreatedInventory))
  (bind _in_slotable_class (Variables|Default|GetIn%20Slotable%20Class))
  (bind _returnvalue (Class|Inventory|GetSlotables _createdinventory))
  (Class|SfTest|GenericAssert (and (== (Utilities|GetClass (Utilities|Array|Get(acopy) _returnvalue)) _in_slotable_class) (== (Utilities|GetClass (Utilities|Array|Get(acopy) _returnvalue 1)) _in_slotable_class)) "Changes synced to client" "Changes failed to sync to client"))

(event Custom|OnAddSlotable
  (params (Slotable :type Slotable%20Object%20Reference))
  (bind _output_get (Variables|Default|SetDelegate%20ref%20added%20slotable Slotable)))

(event Custom|OnRemoveSlotable
  (params (Slotable :type Slotable%20Object%20Reference))
  (bind _output_get (Variables|Default|SetSlotableOnRemoveCalled true)))

(event Custom|Add%20card%20with%20lifetime
  (Class|Inventory|BindonAddSharedCard (Variables|Default|GetCreatedInventory) (Variables|Default|GetIn%20Card%20Class) (delegate Custom|OnAddSharedCard))
  (Class|Inventory|ServerAddSharedCard (Variables|Default|GetCreatedInventory) (Variables|Default|GetIn%20Card%20Class) 0.5)
  (Class|SfTest|AssertBool (Class|Inventory|HasSharedCard (Variables|Default|GetCreatedInventory) (Variables|Default|GetIn%20Card%20Class)) true "Added shared card")
  (Class|SfTest|AssertBool (Variables|Default|GetCard%20added) true "On card added")
  (Class|SfTest|AssertFloat (Class|Inventory|GetSharedCardLifetime (Variables|Default|GetCreatedInventory) (Variables|Default|GetIn%20Card%20Class)) 0.5 0.5 "Lifetime was set"))

(event Custom|OnRemoveSharedCard
  (params (CardClass :type Object%20Class%20Reference) (bIsPredictableContext :type Boolean))
  (Variables|Default|SetCard%20removed true))

(event Custom|OnAddSharedCard
  (params (CardClass :type Object%20Class%20Reference) (bIsPredictableContext :type Boolean))
  (Variables|Default|SetCard%20added true))

(event Custom|Verify%20client%20card%20lifetime%20ended
  (Class|SfTest|AssertBool (Class|Inventory|HasSharedCard (Variables|Default|GetCreatedInventory) (Variables|Default|GetIn%20Card%20Class)) false "Card exists on client after lifetime"))

(event EventBlueprintRegisterProcedures
  (Class|SfTest|AddProcedure (delegate Custom|Create%20form%20pawn%20and%20inventory) "ROLE_Authority" 0.0)
  (Class|SfTest|AddProcedure (delegate Custom|Check%20OwningFormCore%20synced%20to%20client) "ROLE_AutonomousProxy" 0.0)
  (Class|SfTest|AddProcedure (delegate Custom|Check%20default%20slotable%20synced%20to%20client) "ROLE_AutonomousProxy" 0.0)
  (Class|SfTest|AddProcedure (delegate Custom|Add%20slotable) "ROLE_Authority" 0.0)
  (Class|SfTest|AddProcedure (delegate Custom|RemoveSlotableByIndex) "ROLE_Authority" 0.0)
  (Class|SfTest|AddProcedure (delegate Custom|Set%20slotable) "ROLE_Authority" 0.0)
  (Class|SfTest|AddProcedure (delegate Custom|Insert%20slotable) "ROLE_Authority" 0.0)
  (Class|SfTest|AddProcedure (delegate Custom|Try%20GetSlotablesOfClass%20on%20client) "ROLE_AutonomousProxy" 0.0)
  (Class|SfTest|AddProcedure (delegate Custom|Swap%20slotable) "ROLE_Authority" 0.0)
  (Class|SfTest|AddProcedure (delegate Custom|Trade%20slotables%20between%20inventories) "ROLE_Authority" 0.0)
  (Class|SfTest|AddProcedure (delegate Custom|Verify%20changes%20on%20client) "ROLE_AutonomousProxy" 0.0)
  (Class|SfTest|AddProcedure (delegate Custom|Check%20default%20card%20added) "ROLE_AutonomousProxy" 0.0)
  (Class|SfTest|AddProcedure (delegate Custom|Card%20removal) "ROLE_Authority" 0.0)
  (Class|SfTest|AddProcedure (delegate Custom|Add%20card%20with%20lifetime) "ROLE_Authority" 0.8)
  (Class|SfTest|AddProcedure (delegate Custom|Verify%20client%20card%20lifetime%20ended) "ROLE_AutonomousProxy" 0.0))