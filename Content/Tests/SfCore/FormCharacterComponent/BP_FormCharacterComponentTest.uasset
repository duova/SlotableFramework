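; Networked functional test that checks predicted input on a Form character executes a constituent action and reaches other net roles.
; It registers role-targeted procedures: Authority spawns the pawn and caches constituents, the autonomous player's controller possesses it, then the autonomous proxy injects Enhanced Input.
; Assertions read the first dummy predicted constituent's executed flag on Authority and simulated proxy.
; The check labeled "locally" is registered on Authority, not the autonomous proxy.
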(event Custom|Initialize%20FormCharacter
  (bind _returnvalue (Class|SfObject|SpawnActorinOwnerWorld (Variables|Default|GetFormCharacter%20class) (Variables|Default|GetLocation) (Variables|Default|GetRotation)))
  (bind _aspawn (Utilities|Casting|CastToPawn _returnvalue))
  (bind _output_get (Variables|Default|SetFormCharacter _aspawn))
  (Variables|Default|SetFormCoreComp (Actor|GetComponentbyClass _output_get "/Script/SfCore.FormCoreComponent"))
  (Variables|Default|SetConstituent1 (Utilities|Array|Get(acopy) (Class|Slotable|GetConstituents (Utilities|Array|Get(acopy) (Class|Inventory|GetSlotables (Utilities|Array|Get(acopy) (Class|FormCoreComponent|GetInventories (Variables|Default|GetFormCoreComp))))))))
  (Variables|Default|SetConstituent2 (Utilities|Array|Get(acopy) (Class|Slotable|GetConstituents (Utilities|Array|Get(acopy) (Class|Inventory|GetSlotables (Utilities|Array|Get(acopy) (Class|FormCoreComponent|GetInventories (Variables|Default|GetFormCoreComp)))) 1))))
  (Variables|Default|SetConstituent3 (Utilities|Array|Get(acopy) (Class|Slotable|GetConstituents (Utilities|Array|Get(acopy) (Class|Inventory|GetSlotables (Utilities|Array|Get(acopy) (Class|FormCoreComponent|GetInventories (Variables|Default|GetFormCoreComp)))) 2)))))

(event Custom|Verify%20action%20executed%20locally
  (bind _asbp_dummy_predicted_constituent (Utilities|Casting|CastToBP_DummyPredictedConstituent (Variables|Default|GetConstituent1)))
  (Class|SfTest|AssertBool (Variables|/Game/Tests/SfCore/FormCharacterComponent/BP_DummyPredictedConstituent.BP_DummyPredictedConstituent_C|GetInput1ActionExecuted _asbp_dummy_predicted_constituent) true "Input 1 executed action locally."))

(event Custom|Verify%20action%20executed%20on%20server
  (bind _asbp_dummy_predicted_constituent (Utilities|Casting|CastToBP_DummyPredictedConstituent (Variables|Default|GetConstituent1)))
  (Class|SfTest|AssertBool (Variables|/Game/Tests/SfCore/FormCharacterComponent/BP_DummyPredictedConstituent.BP_DummyPredictedConstituent_C|GetInput1ActionExecuted _asbp_dummy_predicted_constituent) true "Input 1 executed action on server."))

(event Custom|Run%20predicted%20input%201
  (bind _asplayer_controller (Utilities|Casting|CastToPlayerController (Pawn|GetController (Variables|Default|GetFormCharacter))))
  (Class|EnhancedInputSubsystemInterface|InjectInputVectorforAction(Message) (PlayerController|LocalPlayerSubsystems|GetEnhancedInputLocalPlayerSubsystem _asplayer_controller) "/Game/Tests/SfCore/FormCharacterComponent/IA_Test1.IA_Test1" "1.000000,0.000000,0.000000"))

(event Custom|Verify%20action%20executed%20on%20simulated%20proxy
  (bind _asbp_dummy_predicted_constituent (Utilities|Casting|CastToBP_DummyPredictedConstituent (Variables|Default|GetConstituent1)))
  (Class|SfTest|AssertBool (Variables|/Game/Tests/SfCore/FormCharacterComponent/BP_DummyPredictedConstituent.BP_DummyPredictedConstituent_C|GetInput1ActionExecuted _asbp_dummy_predicted_constituent) true "Input 1 executed action on simulated client."))

(event Custom|Give%20possession
  (Pawn|Possess (Class|SfTest|GetAutonomousPlayerController) (Variables|Default|GetFormCharacter)))

(event EventBlueprintRegisterProcedures
  (Class|SfTest|AddProcedure (delegate Custom|Initialize%20FormCharacter) "ROLE_Authority" 0.0)
  (Class|SfTest|AddProcedure (delegate Custom|Give%20possession) "ROLE_Authority" 0.0)
  (Class|SfTest|AddProcedure (delegate Custom|Run%20predicted%20input%201) "ROLE_AutonomousProxy" 0.0)
  (Class|SfTest|AddProcedure (delegate Custom|Verify%20action%20executed%20locally) "ROLE_Authority" 0.1)
  (Class|SfTest|AddProcedure (delegate Custom|Verify%20action%20executed%20on%20server) "ROLE_Authority" 0.0)
  (Class|SfTest|AddProcedure (delegate Custom|Verify%20action%20executed%20on%20simulated%20proxy) "ROLE_SimulatedProxy" 0.0))