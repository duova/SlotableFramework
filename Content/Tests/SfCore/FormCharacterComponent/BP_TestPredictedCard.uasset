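; BP_TestPredictedCard is a test card object for the SfCore form character component tests, reporting its own lifecycle to the owning character.
; On Initialize and Deinitialize it follows its owning inventory to the form core's owner and casts that to BP_DummyFormCharacter.
; It then sets CardObjectSpawned or CardObjectDeinitialized to true on that dummy, recording that each event ran.
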(event EventInitialize
  (bind _asbp_dummy_form_character (Utilities|Casting|CastToBP_DummyFormCharacter (Components|GetOwner (Variables|/Script/SfCore.Inventory|GetOwningFormCore (Variables|Default|GetOwningInventory)))))
  (Variables|/Game/Tests/SfCore/FormCharacterComponent/BP_DummyFormCharacter.BP_DummyFormCharacter_C|SetCardObjectSpawned _asbp_dummy_form_character true))

(event EventDeinitialize
  (bind _asbp_dummy_form_character (Utilities|Casting|CastToBP_DummyFormCharacter (Components|GetOwner (Variables|/Script/SfCore.Inventory|GetOwningFormCore (Variables|Default|GetOwningInventory)))))
  (Variables|/Game/Tests/SfCore/FormCharacterComponent/BP_DummyFormCharacter.BP_DummyFormCharacter_C|SetCardObjectDeinitialized _asbp_dummy_form_character true))