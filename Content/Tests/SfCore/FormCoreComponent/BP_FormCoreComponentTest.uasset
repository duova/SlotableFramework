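; Networked automated test for FormCoreComponent, checking team, inventory, view mode and trigger features on a spawned pawn.
; It registers ordered procedures tagged by net role, mostly alternating server changes with autonomous-proxy sync checks.
; Steps cover the default inventory, team setting, inventory addition and removal by index or reference, first/third-person switching, and trigger binding and activation.
; Assertions report each result, and the final step destroys the pawn.
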(event Custom|Create%20form%20pawn
  (bind _returnvalue (Class|SfObject|SpawnActorinOwnerWorld (Variables|Default|GetPawnClass) (Math|Vector|MakeVector 0.0 0.0 0.0) (Math|Rotator|MakeRotator 0.0 0.0 0.0)))
  (bind _output_get (Variables|Default|SetPawn _returnvalue))
  (bind _output_get_2 (Variables|Default|SetFormCore (Actor|GetComponentbyClass _output_get "/Script/SfCore.FormCoreComponent")))
  (Class|SfTest|GenericAssert (Utilities|IsValid (Utilities|Array|Get(acopy) (Class|FormCoreComponent|GetInventories _output_get_2))) "Default inventory successfully created." "Failed to create default inventory.")
  (Class|FormCoreComponent|ServerRemoveInventory (Variables|Default|GetFormCore) (Utilities|Array|Get(acopy) (Class|FormCoreComponent|GetInventories _output_get_2))))

(event Custom|Create%20inventory
  (bind _formcore (Variables|Default|GetFormCore))
  (bind _returnvalue (Class|FormCoreComponent|ServerAddInventory _formcore (Variables|Default|GetIn%20Inventory%20Class)))
  (Variables|Default|SetCreatedInventory _returnvalue)
  (Class|SfTest|GenericAssert (== _returnvalue (Utilities|Array|Get(acopy) (Class|FormCoreComponent|GetInventories _formcore))) "Inventory sucessfully added on server." "Inventory failed to be added on server."))

(event Custom|Check%20remove%20inventory%20by%20ptr%20sync
  (Class|SfTest|AssertInt (Utilities|Array|Length (Class|FormCoreComponent|GetInventories (Variables|Default|GetFormCore))) 0 0 "Check remove inventory by ptr sync"))

(event Custom|Client%20first/third%20person
  (bind _formcore (Variables|Default|GetFormCore))
  (bind _formcore_2 (Variables|Default|GetFormCore))
  (Class|FormCoreComponent|ClientSettoFirstPerson _formcore_2)
  (Class|SfTest|AssertBool (Class|FormCoreComponent|IsFirstPerson _formcore_2) true "Check can change to first person")
  (Class|FormCoreComponent|ClientSettoThirdPerson _formcore)
  (Class|SfTest|AssertBool (Class|FormCoreComponent|IsFirstPerson _formcore) false "Check can change to third person"))

(event Custom|Check%20triggers%20work
  (bind _formcore (Variables|Default|GetFormCore))
  (Class|SfTest|AssertBool (Class|FormCoreComponent|ServerHasTrigger (Variables|Default|GetFormCore) "(TagName=\"Trigger.Test\")") true "Test HasTrigger")
  (Class|FormCoreComponent|ServerBindTrigger _formcore "(TagName=\"Trigger.Test\")" (delegate Custom|Trigger%20binded%20event))
  (Class|FormCoreComponent|ServerActivateTrigger _formcore "(TagName=\"Trigger.Test\")")
  (Class|SfTest|AssertBool (Variables|Default|GetTriggerSuccess) true "Trigger check"))

(event Custom|Trigger%20binded%20event
  (Variables|Default|SetTriggerSuccess true))

(event Custom|Remove%20FormPawn%20before%20ending%20test
  (Actor|DestroyActor (Variables|Default|GetPawn)))

(event Custom|Add%20team
  (bind _formcore (Variables|Default|GetFormCore))
  (Class|FormCoreComponent|ServerSetTeam _formcore "(TagName=\"Team.Test\")")
  (Class|SfTest|GenericAssert (== (Class|FormCoreComponent|GetTeam _formcore) (GameplayTags|MakeLiteralGameplayTag "(TagName=\"Team.Test\")")) "Server add get team succeeded." "Server add get team failed."))

(event Custom|Check%20inventory%20synced%20to%20client
  (Class|SfTest|GenericAssert (== (Variables|Default|GetCreatedInventory) (Utilities|Array|Get(acopy) (Class|FormCoreComponent|GetInventories (Variables|Default|GetFormCore)))) "Inventory sucessfully synced to autonomous client." "Inventory failed to sync to autonomous client."))

(event Custom|Check%20that%20team%20synced%20to%20client
  (bind _formcore (Variables|Default|GetFormCore))
  (Class|FormCoreComponent|ServerSetTeam _formcore "(TagName=\"Team.Test\")")
  (Class|SfTest|GenericAssert (== (Class|FormCoreComponent|GetTeam _formcore) (GameplayTags|MakeLiteralGameplayTag "(TagName=\"Team.Test\")")) "Add get team synced to autonomous proxy." "Add get team failed to sync to autonomous proxy."))

(event Custom|Remove%20inventory
  (Class|FormCoreComponent|ServerRemoveInventorybyIndex (Variables|Default|GetFormCore)))

(event Custom|Check%20remove%20inventory%20by%20index%20sync
  (Class|SfTest|AssertInt (Utilities|Array|Length (Class|FormCoreComponent|GetInventories (Variables|Default|GetFormCore))) 0 0 "Check remove inventory by index sync"))

(event Custom|Add%20and%20remove%20inventory%20to%20check%20second%20removal%20function
  (bind _formcore (Variables|Default|GetFormCore))
  (bind _returnvalue (Class|FormCoreComponent|ServerAddInventory _formcore (Variables|Default|GetIn%20Inventory%20Class)))
  (Class|FormCoreComponent|ServerRemoveInventory _formcore _returnvalue))

(event EventBlueprintRegisterProcedures
  (Class|SfTest|AddProcedure (delegate Custom|Create%20form%20pawn) "ROLE_Authority" 0.0)
  (Class|SfTest|AddProcedure (delegate Custom|Add%20team) "ROLE_Authority" 0.0)
  (Class|SfTest|AddProcedure (delegate Custom|Check%20that%20team%20synced%20to%20client) "ROLE_AutonomousProxy" 0.0)
  (Class|SfTest|AddProcedure (delegate Custom|Create%20inventory) "ROLE_Authority" 0.0)
  (Class|SfTest|AddProcedure (delegate Custom|Check%20inventory%20synced%20to%20client) "ROLE_AutonomousProxy" 0.0)
  (Class|SfTest|AddProcedure (delegate Custom|Remove%20inventory) "ROLE_Authority" 0.0)
  (Class|SfTest|AddProcedure (delegate Custom|Check%20remove%20inventory%20by%20index%20sync) "ROLE_AutonomousProxy" 0.0)
  (Class|SfTest|AddProcedure (delegate Custom|Add%20and%20remove%20inventory%20to%20check%20second%20removal%20function) "ROLE_Authority" 0.0)
  (Class|SfTest|AddProcedure (delegate Custom|Check%20remove%20inventory%20by%20ptr%20sync) "ROLE_AutonomousProxy" 0.0)
  (Class|SfTest|AddProcedure (delegate Custom|Client%20first/third%20person) "ROLE_AutonomousProxy" 0.0)
  (Class|SfTest|AddProcedure (delegate Custom|Check%20triggers%20work) "ROLE_Authority" 0.0)
  (Class|SfTest|AddProcedure (delegate Custom|Remove%20FormPawn%20before%20ending%20test) "ROLE_None" 0.0))