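; Multi-role network test for FormCoreComponent, covering team assignment and inventory creation.
; Registered procedures run per net role: authority spawns a pawn, sets its team and adds an inventory, while autonomous and simulated proxies assert each result.
; Pawn, component and inventory references are marked dirty for replication.
; Proxy team checks call ServerSetTeam again before asserting; inventory checks only compare the first entry.
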(event Custom|Create%20form%20pawn
  (bind _returnvalue (Class|SfObject|SpawnActorinOwnerWorld (Variables|Default|GetPawnClass) (Math|Vector|MakeVector 0.0 0.0 0.0) (Math|Rotator|MakeRotator 0.0 0.0 0.0)))
  (bind _output_get (Variables|Default|SetPawn _returnvalue))
  (Variables|Default|SetFormCore (Actor|GetComponentbyClass _output_get "/Script/SfCore.FormCoreComponent"))
  (Class|NetPushModelHelpers|MarkPropertyDirty "BP_FormCoreComponentTest" "Form Core")
  (Class|NetPushModelHelpers|MarkPropertyDirty "BP_FormCoreComponentTest" "Pawn"))

(event Custom|Create%20inventory
  (bind _formcore (Variables|Default|GetFormCore))
  (bind _returnvalue (Class|FormCoreComponent|ServerAddInventory _formcore (Variables|Default|GetIn%20Inventory%20Class)))
  (Variables|Default|SetCreatedInventory _returnvalue)
  (Class|NetPushModelHelpers|MarkPropertyDirty "BP_FormCoreComponentTest" "CreatedInventory")
  (Class|SfTest|GenericAssert (== _returnvalue (Utilities|Array|Get(acopy) (Class|FormCoreComponent|GetInventories _formcore))) "Inventory sucessfully added on server." "Inventory failed to be added on server."))

(event Custom|Add%20team
  (bind _formcore (Variables|Default|GetFormCore))
  (Class|FormCoreComponent|ServerSetTeam _formcore "(TagName=\"Team.Test\")")
  (Class|SfTest|GenericAssert (== (Class|FormCoreComponent|GetTeam _formcore) (GameplayTags|MakeLiteralGameplayTag "(TagName=\"Team.Test\")")) "Server add get team succeeded." "Server add get team failed."))

(event Custom|Check%20inventory%20synced%20to%20autonomous%20proxy
  (Class|SfTest|GenericAssert (== (Variables|Default|GetCreatedInventory) (Utilities|Array|Get(acopy) (Class|FormCoreComponent|GetInventories (Variables|Default|GetFormCore)))) "Inventory sucessfully synced to autonomous client." "Inventory failed to sync to autonomous client."))

(event Custom|Check%20that%20team%20synced%20to%20autonomous%20proxy
  (bind _formcore (Variables|Default|GetFormCore))
  (Class|FormCoreComponent|ServerSetTeam _formcore "(TagName=\"Team.Test\")")
  (Class|SfTest|GenericAssert (== (Class|FormCoreComponent|GetTeam _formcore) (GameplayTags|MakeLiteralGameplayTag "(TagName=\"Team.Test\")")) "Add get team synced to autonomous proxy." "Add get team failed to sync to autonomous proxy."))

(event Custom|Check%20that%20team%20synced%20to%20simulated%20proxy
  (bind _formcore (Variables|Default|GetFormCore))
  (Class|FormCoreComponent|ServerSetTeam _formcore "(TagName=\"Team.Test\")")
  (Class|SfTest|GenericAssert (== (Class|FormCoreComponent|GetTeam _formcore) (GameplayTags|MakeLiteralGameplayTag "(TagName=\"Team.Test\")")) "Add get team synced to simulated proxy." "Add get team failed to sync to simulated proxy."))

(event Custom|Check%20inventory%20synced%20to%20simulated%20proxy
  (Class|SfTest|GenericAssert (== (Variables|Default|GetCreatedInventory) (Utilities|Array|Get(acopy) (Class|FormCoreComponent|GetInventories (Variables|Default|GetFormCore)))) "Inventory sucessfully synced to simulated client." "Inventory failed to sync to simulated client."))

(event EventBlueprintRegisterProcedures
  (Class|SfTest|AddProcedure (delegate Custom|Create%20form%20pawn) "ROLE_Authority" 0.0)
  (Class|SfTest|AddProcedure (delegate Custom|Add%20team) "ROLE_Authority" 0.0)
  (Class|SfTest|AddProcedure (delegate Custom|Check%20that%20team%20synced%20to%20autonomous%20proxy) "ROLE_AutonomousProxy" 0.0)
  (Class|SfTest|AddProcedure (delegate Custom|Check%20that%20team%20synced%20to%20simulated%20proxy) "ROLE_SimulatedProxy" 0.0)
  (Class|SfTest|AddProcedure (delegate Custom|Create%20inventory) "ROLE_Authority" 0.0)
  (Class|SfTest|AddProcedure (delegate Custom|Check%20inventory%20synced%20to%20autonomous%20proxy) "ROLE_AutonomousProxy" 0.0)
  (Class|SfTest|AddProcedure (delegate Custom|Check%20inventory%20synced%20to%20simulated%20proxy) "ROLE_SimulatedProxy" 0.0))