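; Multiplayer test for SlotableConstituent, checking that slotables replicate and constituent actions execute across net roles.
; Registers ordered procedures, each bound to authority, autonomous proxy or simulated proxy.
; Authority spawns a pawn with a FormCore inventory, adds a slotable and has the autonomous player controller possess the pawn.
; After the autonomous proxy verifies replication, authority fires a dummy constituent's action, with asserts confirming the call on server, autonomous and simulated roles.
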(event Custom|Create%20form%20pawn%20and%20inventory
  (bind _returnvalue (Class|SfObject|SpawnActorinOwnerWorld (Variables|Default|GetPawnClass) (Math|Vector|MakeVector 0.0 0.0 0.0) (Math|Rotator|MakeRotator 0.0 0.0 0.0)))
  (bind _aspawn (Utilities|Casting|CastToPawn _returnvalue))
  (bind _output_get (Variables|Default|SetPawn _aspawn))
  (bind _output_get_2 (Variables|Default|SetFormCore (Actor|GetComponentbyClass _output_get "/Script/SfCore.FormCoreComponent")))
  (Class|SfTest|GenericAssert (Utilities|IsValid (Utilities|Array|Get(acopy) (Class|FormCoreComponent|GetInventories _output_get_2))) "Default inventory successfully created." "Failed to create default inventory.")
  (bind _returnvalue_2 (Class|FormCoreComponent|ServerAddInventory (Variables|Default|GetFormCore) (Variables|Default|GetIn%20Inventory%20Class)))
  (bind _output_get_3 (Variables|Default|SetCreatedInventory _returnvalue_2))
  (Class|Inventory|ServerRemoveSlotablebyIndex _output_get_3 0 true))

(event Custom|Verify%20slotable%20replication
  (bind _createdinventory (Variables|Default|GetCreatedInventory))
  (bind _returnvalue (Class|Inventory|GetSlotables _createdinventory))
  (Class|SfTest|AssertInt (Utilities|Array|Length _returnvalue) 1 1 "Slotable added")
  (Class|SfTest|AssertBool (Utilities|IsValid (Utilities|Array|Get(acopy) (Class|Slotable|GetConstituents (Utilities|Array|Get(acopy) _returnvalue)))) true "Constituent added"))

(event Custom|Call%20action
  (bind _asbp_dummy_constituent (Utilities|Casting|CastToBP_DummyConstituent (Utilities|Array|Get(acopy) (Class|Slotable|GetConstituentsOfClass (Variables|Default|GetCreated%20slotable) (Variables|Default|GetIn%20Constituent%20Class)))))
  (bind _output_get (Variables|Default|SetCreatedConstituent _asbp_dummy_constituent))
  (Default|CallExecuteActionDelegate _output_get)
  (Class|SfTest|AssertBool (Variables|/Game/Tests/SfCore/SlotableConstituent/BP_DummyConstituent.BP_DummyConstituent_C|GetAction%20called%20on%20server (Variables|Default|GetCreatedConstituent)) true "Action called on server")
  (Class|SfTest|AssertBool (Variables|/Game/Tests/SfCore/SlotableConstituent/BP_DummyConstituent.BP_DummyConstituent_C|GetEvent%20called (Variables|Default|GetCreatedConstituent)) true "Blueprint event for action called"))

(event Custom|Check%20action%20on%20autonomous
  (Class|SfTest|AssertBool (Variables|/Game/Tests/SfCore/SlotableConstituent/BP_DummyConstituent.BP_DummyConstituent_C|GetAction%20called%20on%20autonomous (Variables|Default|GetCreatedConstituent)) true "Action called on autonomous"))

(event Custom|Check%20action%20on%20simulated
  (Class|SfTest|AssertBool (Variables|/Game/Tests/SfCore/SlotableConstituent/BP_DummyConstituent.BP_DummyConstituent_C|GetAction%20called%20on%20simulated (Variables|Default|GetCreatedConstituent)) true "Action called on simulated"))

(event Custom|Add%20slotable%20and%20give%20owner%20possession
  (bind _returnvalue (Class|Inventory|ServerAddSlotable (Variables|Default|GetCreatedInventory) (Variables|Default|GetIn%20Slotable%20Class)))
  (Variables|Default|SetCreated%20slotable _returnvalue)
  (Pawn|Possess (Class|SfTest|GetAutonomousPlayerController) (Variables|Default|GetPawn)))

(event EventBlueprintRegisterProcedures
  (Class|SfTest|AddProcedure (delegate Custom|Create%20form%20pawn%20and%20inventory) "ROLE_Authority" 0.0)
  (Class|SfTest|AddProcedure (delegate Custom|Add%20slotable%20and%20give%20owner%20possession) "ROLE_Authority" 0.0)
  (Class|SfTest|AddProcedure (delegate Custom|Verify%20slotable%20replication) "ROLE_AutonomousProxy" 0.0)
  (Class|SfTest|AddProcedure (delegate Custom|Call%20action) "ROLE_Authority" 0.0)
  (Class|SfTest|AddProcedure (delegate Custom|Check%20action%20on%20autonomous) "ROLE_AutonomousProxy" 0.0)
  (Class|SfTest|AddProcedure (delegate Custom|Check%20action%20on%20simulated) "ROLE_SimulatedProxy" 0.0))